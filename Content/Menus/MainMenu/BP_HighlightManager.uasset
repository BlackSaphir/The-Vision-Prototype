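; BP_HighlightManager outlines ammo items, Berettas and alarm buttons when the player character is nearby.
; Every Tick, it gathers all actors of each class and compares their distance to the player against a fixed threshold.
; Closer actors get custom depth rendering with a shared stencil value, and farther ones have it disabled.
; Alarm buttons only receive the highlight while unpressed.
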(event `self.ReceiveTick`
  (params (DeltaSeconds :type "Float (single-precision)"))
  (bind _returnvalue (`GameplayStatics.GetPlayerCharacter` 0))
  (`|ExecutionSequence`
    (:`then_0`
      ;[1 1 1] Ammo Outline
      (bind _outactors (`GameplayStatics.GetAllActorsOfClass` "/Game/Blueprints/GameplayActor/BP_Item_Ammo.BP_Item_Ammo_C"))
      (for _array_element _outactors
        (`/Engine/EditorBlueprintResources/StandardMacros.IsValid` _returnvalue
          (:`Is Valid`
            (`/Engine/EditorBlueprintResources/StandardMacros.IsValid` (`GameplayStatics.GetPlayerCharacter` 0)
              (:`Is Valid`
                (`/Engine/EditorBlueprintResources/StandardMacros.CompareFloat` (`self.GetDistanceTo` _array_element _returnvalue) 500.0
                  (:`>`
                    (`PrimitiveComponent.SetRenderCustomDepth` (`/Game/Blueprints/GameplayActor/BP_Item_Ammo.Cube` _array_element) false))
                  (:`<`
                    (bind _cube (`/Game/Blueprints/GameplayActor/BP_Item_Ammo.Cube` _array_element))
                    (`PrimitiveComponent.SetCustomDepthStencilValue` _cube 252)
                    (`PrimitiveComponent.SetRenderCustomDepth` _cube true)))))))))
    (:`then_1`
      ;[1 1 1] Beretta Outline
      (bind _outactors_2 (`GameplayStatics.GetAllActorsOfClass` "/Game/Blueprints/GameplayActor/BP_Beretta.BP_Beretta_C"))
      (for _array_element_2 _outactors_2
        (`/Engine/EditorBlueprintResources/StandardMacros.IsValid` _array_element_2
          (:`Is Valid`
            (`/Engine/EditorBlueprintResources/StandardMacros.IsValid` (`GameplayStatics.GetPlayerCharacter` 0)
              (:`Is Valid`
                (`/Engine/EditorBlueprintResources/StandardMacros.CompareFloat` (`self.GetDistanceTo` _array_element_2 (`GameplayStatics.GetPlayerCharacter` 0)) 500.0
                  (:`>`
                    (`PrimitiveComponent.SetRenderCustomDepth` (`/Game/Blueprints/GameplayActor/BP_Beretta.StaticMesh` _array_element_2) false))
                  (:`<`
                    (`PrimitiveComponent.SetCustomDepthStencilValue` (`/Game/Blueprints/GameplayActor/BP_Beretta.StaticMesh` _array_element_2) 252)
                    (`PrimitiveComponent.SetRenderCustomDepth` (`/Game/Blueprints/GameplayActor/BP_Beretta.StaticMesh` _array_element_2) true)))))))))
    (:`then_2`
      ;[1 1 1] AlarmButton Outline
      (bind _outactors_3 (`GameplayStatics.GetAllActorsOfClass` "/Game/Blueprints/GameplayActor/BP_AlarmButton.BP_AlarmButton_C"))
      (for _array_element_3 _outactors_3
        (`/Engine/EditorBlueprintResources/StandardMacros.IsValid` _array_element_3
          (:`Is Valid`
            (`/Engine/EditorBlueprintResources/StandardMacros.IsValid` (`GameplayStatics.GetPlayerCharacter` 0)
              (:`Is Valid`
                (`/Engine/EditorBlueprintResources/StandardMacros.CompareFloat` (`self.GetDistanceTo` _array_element_3 (`GameplayStatics.GetPlayerCharacter` 0)) 500.0
                  (:`>`
                    (`PrimitiveComponent.SetRenderCustomDepth` (`/Game/Blueprints/GameplayActor/BP_AlarmButton.Button` _array_element_3) false))
                  (:`<`
                    (if (not (`/Game/Blueprints/GameplayActor/BP_AlarmButton.ButtonPressed` _array_element_3))
                      (`PrimitiveComponent.SetCustomDepthStencilValue` (`/Game/Blueprints/GameplayActor/BP_AlarmButton.Button` _array_element_3) 252)
                      (`PrimitiveComponent.SetRenderCustomDepth` (`/Game/Blueprints/GameplayActor/BP_AlarmButton.Button` _array_element_3) true))))))))))))

(fn `UserConstructionScript`)