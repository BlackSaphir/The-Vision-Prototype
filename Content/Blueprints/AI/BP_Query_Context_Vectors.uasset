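; EQS query context that supplies a set of world locations to environment queries.
; ProvideLocationsSet clears its cached arrays, fetches every actor with GetAllActorsOfClass on the base Actor class, stores each one, and returns their locations.
; The querier inputs are unused, so each call scans the whole world unfiltered and yields the same set regardless of who runs the query.
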(fn `ProvideLocationsSet`
  (params (QuerierObject :type "Object Object Reference") (QuerierActor :type "Actor Object Reference"))
  (returns (ResultingLocationSet :type "Array of Vector Structure"))
  (locals (verctors :type "Array of Vector Structure"))
  (`KismetArrayLibrary.Array_Clear` (`local.verctors`))
  (`KismetArrayLibrary.Array_Clear` (`self.Actors_Context`))
  (bind _outactors (`GameplayStatics.GetAllActorsOfClass` "/Script/Engine.Actor"))
  (for _array_element _outactors
    (`KismetArrayLibrary.Array_Add` (`self.Actors_Context`) _array_element)
    (`KismetArrayLibrary.Array_Add` (`local.verctors`) (`Actor.K2_GetActorLocation` _array_element)))
  (return (`local.verctors`)))