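; BP_Mutant_Enemy is a mutant enemy actor that serves as a brief, one-shot apparition.
; Its mesh is hidden on BeginPlay until the Appear event shows it, then the actor destroys itself after a half-second delay.
; Nothing in this graph calls Appear.
; Unconnected nodes would rotate the mesh toward the player with a yaw offset, but Tick is empty, so they never run.
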(event `self.ReceiveBeginPlay`
  (`SceneComponent.SetHiddenInGame` (`self.Mesh`) true false))

(event `Appear`
  (`SceneComponent.SetHiddenInGame` (`self.Mesh`) false false)
  (`KismetSystemLibrary.Delay` 0.5)
  (`self.K2_DestroyActor`))

(event `self.ReceiveTick`
  (params (DeltaSeconds :type "Float (single-precision)")))

(fn `UserConstructionScript`)