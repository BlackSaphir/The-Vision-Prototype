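; EQS context that supplies navmesh-projected positions derived from traces around actors near the querier.
; It traces Visibility from radial spokes around each nearby actor toward the querier; misses feed a debug-drawn Camera trace offset from the first hit result.
; When that second trace hits, the offset point is projected to navigation and stored.
; FoundActors latches on the first stored position, blocking later searches.
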(fn `ProvideLocationsSet`
  (params (QuerierObject :type "Object Object Reference") (QuerierActor :type "Actor Object Reference"))
  (returns (ResultingLocationSet :type "Array of Vector Structure"))
  (locals (Positions :type "Array of Vector Structure") (Actors :type "Array of Actor Object Reference") (found_Actors :type Boolean) (`distance to querier` :type "Float (double-precision)" :default 5000.0))
  (bind _offsetfromwall (`self.OffsetFromWall`))
  (bind _numberofspokes (`self.NumberOfSpokes`))
  (bind _returnvalue (`Actor.K2_GetActorLocation` (`local.QuerierActor`)))
  (`KismetArrayLibrary.Array_Clear` (`local.Positions`))
  (`KismetArrayLibrary.Array_Clear` (`local.Actors`))
  (if (not (`local.found_Actors`))
    (bind _outactors (`GameplayStatics.GetAllActorsOfClass` "/Script/Engine.Actor"))
    (for _array_element _outactors
      (if (< (`Actor.GetDistanceTo` (`local.QuerierActor`) _array_element) (`local.distance to querier`))
        (`KismetArrayLibrary.Array_Add` (`local.Actors`) _array_element)))
    (for _array_element_2 (`local.Actors`)
      (for _index (range _numberofspokes)
        (bind (_outhit _returnvalue_2) (`KismetSystemLibrary.LineTraceSingle` :`Start` (+ (* (`KismetMathLibrary.GreaterGreater_VectorRotator` (1.0 0.0 0.0) (`KismetMathLibrary.MakeRotator` 0.0 0.0 (* _index (/ 360.0 (`KismetMathLibrary.Conv_IntToDouble` _numberofspokes))))) (`self.Radius`)) (`Actor.K2_GetActorLocation` _array_element_2)) :`End` _returnvalue :`TraceChannel` "TraceTypeQuery1" :`DrawTime` 10.0))
        (if (not _returnvalue_2)
          (bind (_bblockinghit _binitialoverlap _time _location _impactpoint _normal) (`GameplayStatics.BreakHitResult` _outhit))
          (bind (_outhit_2 _returnvalue_3) (`KismetSystemLibrary.LineTraceSingle` :`Start` (+ _impactpoint (* (* _normal -1.0) _offsetfromwall)) :`End` _returnvalue :`TraceChannel` "TraceTypeQuery2" :`DrawDebugType` "ForDuration" :`DrawTime` 10.0))
          (if _returnvalue_3
            (`KismetArrayLibrary.Array_Add` (`local.Positions`) (`NavigationSystem.K2_ProjectPointToNavigation` (+ _impactpoint (* _normal _offsetfromwall)) null "/Script/Engine.RecastFilter_UseDefaultArea"))
            (set `local.found_Actors` true)))))
    (return (`local.Positions`))))