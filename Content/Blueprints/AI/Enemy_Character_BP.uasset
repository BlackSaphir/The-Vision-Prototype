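; Enemy AI character Blueprint that holds the stance and aiming state for its animations.
; FlipFlop-driven toggle events switch crouch, stand guard and aim, with crouch and stand guard each blocked while the other is active.
; While aiming, Tick caches the right-hand IK socket's component-space location to update the animation.
; Unconnected logic for stepping vertical and horizontal aim values remains in the graph but never runs.
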(event `self.ReceiveTick`
  (params (DeltaSeconds :type "Float (single-precision)"))
  (bind _returnvalue_location (`KismetMathLibrary.BreakTransform` (`SceneComponent.GetSocketTransform` (`self.Mesh`) "rhand_ik_socket" "RTS_Component")))
  ;[1 1 1] Updating Socket location of the hand to update the animation
  (if (`self.aim`)
    (set `self.rHandSocket_Loc` _returnvalue_location)))

(event `CrouchToggled`
  ;[1 1 1] Events for AI Animations
  (if (not (`self.standGuard`))
    (`/Engine/EditorBlueprintResources/StandardMacros.FlipFlop`
      (:`A`
        (`self.Crouch`))
      (:`B`
        (`self.UnCrouch`)))))

(event `StandGuardToggle`
  ;[1 1 1] Events for AI Animations
  (if (not (`NavMovementComponent.IsCrouching` (`self.CharacterMovement`)))
    (`/Engine/EditorBlueprintResources/StandardMacros.FlipFlop`
      (:`A`
        (set `self.standGuard` true))
      (:`B`
        (set `self.standGuard` false)))))

(event `AimingToggled`
  ;[1 1 1] Events for AI Animations
  (`/Engine/EditorBlueprintResources/StandardMacros.FlipFlop`
    (:`A`
      (set `self.aim` true))
    (:`B`
      (set `self.aim` false))))

(fn `UserConstructionScript`)