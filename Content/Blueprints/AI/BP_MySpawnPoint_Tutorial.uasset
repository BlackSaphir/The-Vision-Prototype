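; Tutorial spawn point that runs a timed, one-off sequence of enemy AI spawns at its own location and rotation.
; SetSpawnBoolTrueTutorial sets MaySpawnTutorial and passes a DoOnce gate to spawn an Enemy_Character_BP.
; Fixed delays then destroy that enemy, spawn a second one after a short pause, and destroy it too.
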(event `self.SetSpawnBoolTrue_Tutorial`
  (set `self.MaySpawn_Tutorial` true)
  (if (`self.MaySpawn_Tutorial`)
    (`/Engine/EditorBlueprintResources/StandardMacros.DoOnce` false
      (:`Completed`
        (bind _returnvalue (`AIBlueprintHelperLibrary.SpawnAIFromClass` "/Game/Blueprints/AI/Enemy_Character_BP.Enemy_Character_BP_C" null (`self.K2_GetActorLocation`) (`self.K2_GetActorRotation`)))
        (`KismetSystemLibrary.Delay` 11.0)
        (`self.K2_DestroyActor` _returnvalue)
        (`KismetSystemLibrary.Delay` 2.0)
        (bind _returnvalue_2 (`AIBlueprintHelperLibrary.SpawnAIFromClass` "/Game/Blueprints/AI/Enemy_Character_BP.Enemy_Character_BP_C" null (`self.K2_GetActorLocation`) (`self.K2_GetActorRotation`)))
        (`KismetSystemLibrary.Delay` 10.0)
        (`self.K2_DestroyActor` _returnvalue_2)))))

(fn `UserConstructionScript`)