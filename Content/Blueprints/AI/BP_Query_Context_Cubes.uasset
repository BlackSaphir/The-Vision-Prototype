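; An EQS query context that supplies navmesh locations beside obstacles around the querier, apparently as cover candidates.
; It traces inward from evenly spaced spokes on a radius, rotated by pitch only, ignoring FirstPersonCharacter actors.
; For each hit, a Camera-channel trace from behind the impact must also be blocked on its way to the querier.
; Passing impacts are offset along the surface normal and projected onto navigation.
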(fn `ProvideLocationsSet`
  (params (QuerierObject :type "Object Object Reference") (QuerierActor :type "Actor Object Reference"))
  (returns (ResultingLocationSet :type "Array of Vector Structure"))
  (bind _returnvalue (`Actor.K2_GetActorLocation` QuerierActor))
  (bind _numberofspokes (`self.NumberOfSpokes`))
  (bind _offsetfromwall (`self.OffsetFromWall`))
  (bind _outactors (`GameplayStatics.GetAllActorsOfClass` "/Game/Blueprints/Character/FirstPersonCharacter.FirstPersonCharacter_C"))
  (`KismetArrayLibrary.Array_Clear` (`self.LocationSet`))
  (for _index (range _numberofspokes)
    (bind (_outhit _returnvalue_2) (`KismetSystemLibrary.LineTraceSingle` (+ (* (`KismetMathLibrary.GreaterGreater_VectorRotator` (1.0 0.0 0.0) (`KismetMathLibrary.MakeRotator` 0.0 (* _index (/ 360.0 (`KismetMathLibrary.Conv_IntToDouble` _numberofspokes))))) (`self.Radius`)) _returnvalue) _returnvalue "TraceTypeQuery1" false _outactors))
    (if _returnvalue_2
      (bind (_bblockinghit _binitialoverlap _time _location _impactpoint _normal) (`GameplayStatics.BreakHitResult` _outhit))
      (bind (_outhit_2 _returnvalue_3) (`KismetSystemLibrary.LineTraceSingle` (+ (* (* _normal -1.0) _offsetfromwall) _impactpoint) _returnvalue "TraceTypeQuery2"))
      (if _returnvalue_3
        (`KismetArrayLibrary.Array_Add` (`self.LocationSet`) (`NavigationSystem.K2_ProjectPointToNavigation` (+ (* _normal _offsetfromwall) _impactpoint) null "/Script/Engine.RecastFilter_UseDefaultArea")))))
  (for _array_element (`self.LocationSet`)
    (`EnvQueryGenerator_BlueprintBase.AddGeneratedVector` _array_element))
  (return))