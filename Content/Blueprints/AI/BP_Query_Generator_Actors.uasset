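; An EQS generator that, despite its name, produces wall-adjacent navigation points, apparently cover candidates, around each context location.
; It spaces spokes on a radius and traces Visibility from each toward the querier.
; On a hit, a second Camera trace runs to the querier from the opposite side of the hit surface's offset.
; If that also hits, the wall-offset point is projected to the navmesh and added, with debug traces and prints left in.
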(fn `DoItemGeneration`
  (params (ContextLocations :type "Array of Vector Structure (by ref)"))
  (locals (NumberOfSpokes :type Integer :default 10))
  (bind _offsetfromwall (`self.OffsetFromWall`))
  (bind _numberofspokes (`local.NumberOfSpokes`))
  (for _array_element ContextLocations
    (`KismetSystemLibrary.PrintString` (`KismetStringLibrary.Conv_VectorToString` _array_element))
    (bind _asactor (cast `Actor` (`self.GetQuerier`))
      (:`then`
        (for _index (range _numberofspokes)
          (bind _returnvalue (`Actor.K2_GetActorLocation` _asactor))
          (bind (_outhit _returnvalue_2) (`KismetSystemLibrary.LineTraceSingle` :`Start` (+ (* (`KismetMathLibrary.GreaterGreater_VectorRotator` (1.0 0.0 0.0) (`KismetMathLibrary.MakeRotator` 0.0 0.0 (* _index (/ 360.0 (`KismetMathLibrary.Conv_IntToDouble` _numberofspokes))))) (`self.Radius`)) _array_element) :`End` _returnvalue :`TraceChannel` "TraceTypeQuery1" :`DrawDebugType` "ForDuration" :`DrawTime` 10.0))
          (if _returnvalue_2
            (bind (_bblockinghit _binitialoverlap _time _location _impactpoint _normal) (`GameplayStatics.BreakHitResult` _outhit))
            (bind (_outhit_2 _returnvalue_3) (`KismetSystemLibrary.LineTraceSingle` :`Start` (+ _impactpoint (* (* _normal -1.0) _offsetfromwall)) :`End` _returnvalue :`TraceChannel` "TraceTypeQuery2" :`DrawDebugType` "ForDuration" :`DrawTime` 10.0))
            (if _returnvalue_3
              (`self.AddGeneratedVector` (`NavigationSystem.K2_ProjectPointToNavigation` (+ _impactpoint (* _normal _offsetfromwall)) null "/Script/Engine.RecastFilter_UseDefaultArea"))
              (else
                (`KismetSystemLibrary.PrintString` "2 cast"))))))
      (:`CastFailed`
        (`KismetSystemLibrary.PrintString` "actor"))))
  (return))