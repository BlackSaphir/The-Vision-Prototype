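; Enemy spawn point that spawns one Enemy_Character_BP at its own location and rotation when the player's danger level reaches 1.
; Tick casts the player to The_VisionCharacter and checks Gefaehrlichkeitsstufe (danger level).
; A DoOnce that is never reset limits SpawnAI to a single call.
; The Delay after spawning leads nowhere, and the MaySpawn assignment is unconnected.
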(event `self.ReceiveTick`
  (params (DeltaSeconds :type "Float (single-precision)"))
  (bind _asthe_vision_character (cast `The_VisionCharacter` (`GameplayStatics.GetPlayerCharacter` 0)))
  (if (== (`The_VisionCharacter.Gefaehrlichkeitsstufe` _asthe_vision_character) 1)
    (`/Engine/EditorBlueprintResources/StandardMacros.DoOnce` false
      (:`Completed`
        (`self.SpawnAI`)))))

(event `SpawnAI`
  (`AIBlueprintHelperLibrary.SpawnAIFromClass` "/Game/Blueprints/AI/Enemy_Character_BP.Enemy_Character_BP_C" null (`self.K2_GetActorLocation`) (`self.K2_GetActorRotation`))
  (`KismetSystemLibrary.Delay` 2.0))

(fn `UserConstructionScript`)