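; AI spawn point actor that spawns an Enemy_Character_BP at its own location and rotation once activated.
; SetSpawnBoolTrue sets MaySpawn and passes through a DoOnce, so the sequence runs only on the first trigger.
; The first enemy is destroyed after a fixed delay, then a replacement spawns after a short pause and is left in the world.
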(event `self.SetSpawnBoolTrue`
  (set `self.MaySpawn` true)
  (if (`self.MaySpawn`)
    (`/Engine/EditorBlueprintResources/StandardMacros.DoOnce` false
      (:`Completed`
        (bind _returnvalue (`AIBlueprintHelperLibrary.SpawnAIFromClass` "/Game/Blueprints/AI/Enemy_Character_BP.Enemy_Character_BP_C" null (`self.K2_GetActorLocation`) (`self.K2_GetActorRotation`)))
        (`KismetSystemLibrary.Delay` 11.0)
        (`self.K2_DestroyActor` _returnvalue)
        (`KismetSystemLibrary.Delay` 2.0)
        (`AIBlueprintHelperLibrary.SpawnAIFromClass` "/Game/Blueprints/AI/Enemy_Character_BP.Enemy_Character_BP_C" null (`self.K2_GetActorLocation`) (`self.K2_GetActorRotation`))))))

(fn `UserConstructionScript`)