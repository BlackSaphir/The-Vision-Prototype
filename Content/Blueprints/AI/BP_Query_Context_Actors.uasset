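; BP_Query_Context_Actors is an EQS query context that supplies reference locations taken from static mesh actors in the level.
; ProvideLocationsSet gets all StaticMeshActors, but returns inside the loop, so it prints the first actor's name and yields only that location.
; ProvideActorsSet is empty, with an unconnected draft that would print a name and return all actors.
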(fn `ProvideActorsSet`
  (params (QuerierObject :type "Object Object Reference") (QuerierActor :type "Actor Object Reference"))
  (returns (ResultingActorsSet :type "Array of Actor Object Reference")))

(fn `ProvideLocationsSet`
  (params (QuerierObject :type "Object Object Reference") (QuerierActor :type "Actor Object Reference"))
  (returns (ResultingLocationSet :type "Array of Vector Structure"))
  (bind _outactors (`GameplayStatics.GetAllActorsOfClass` "/Script/Engine.StaticMeshActor"))
  (for _array_element _outactors
    (`KismetSystemLibrary.PrintString` (`KismetSystemLibrary.GetDisplayName` _array_element))
    (return (`|MakeArray` (`Actor.K2_GetActorLocation` _array_element)))))