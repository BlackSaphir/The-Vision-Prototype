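; BP_VisionTrigger is a one-shot overlap trigger that plays "The Vision" cutscene and activates AI spawning.
; On overlap it locks player input, clears widgets, plays a sound and starts the camera's vision effect.
; After a delay it flags all AI_SpawnPoint actors to spawn and switches the view to that camera.
; Timed delays then return the view to the pawn, reverse the effect, restore input and re-add the HUD interface.
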(event `self.CollisionComponent.OnComponentBeginOverlap`
  (params (OverlappedComponent :type "PrimitiveComponent Object Reference") (OtherActor :type "Actor Object Reference") (OtherComp :type "PrimitiveComponent Object Reference") (OtherBodyIndex :type Integer) (bFromSweep :type Boolean) (SweepResult :type "HitResult Structure (by ref)"))
  (bind _returnvalue (`GameplayStatics.GetPlayerController` 0))
  (bind _returnvalue_2 (`GameplayStatics.GetPlayerController` 0))
  (bind _returnvalue_3 (`GameplayStatics.GetPlayerController` 0))
  (`/Engine/EditorBlueprintResources/StandardMacros.DoOnce` false
    (:`Completed`
      (`Controller.SetIgnoreMoveInput` _returnvalue_2 true)
      (`Controller.SetIgnoreLookInput` _returnvalue_2 true)
      (`WidgetLayoutLibrary.RemoveAllWidgets`)
      (`GameplayStatics.PlaySoundAtLocation` "/Game/Audio/The_Vision_ViewChange.The_Vision_ViewChange" (`SceneComponent.RelativeLocation` (`self.CollisionComponent`)))
      (`/Game/Blueprints/GameplayActor/Second_Camera_Blueprint.The_Vision` (`self.Camera`))
      (bind _outactors (`GameplayStatics.GetAllActorsOfClass` "/Game/Blueprints/AI/AI_SpawnPoint.AI_SpawnPoint_C"))
      (`KismetSystemLibrary.Delay` 2.0)
      (`/Game/Blueprints/AI/AI_SpawnPoint.SetSpawnBoolTrue` _outactors)
      (`PlayerController.SetViewTargetWithBlend` (`GameplayStatics.GetPlayerController` 0) (`self.Camera`) 0.0 "VTBlend_Linear" 0.0 false)
      (`/Game/Blueprints/GameplayActor/Second_Camera_Blueprint.Play_Ambience_Camera_ViewChange` (`self.Camera`))
      (`KismetSystemLibrary.Delay` 10.0)
      (`/Game/Blueprints/GameplayActor/Second_Camera_Blueprint.Play_ChangeOut_Sound` (`self.Camera`))
      (`PlayerController.SetViewTargetWithBlend` _returnvalue_3 (`Controller.K2_GetPawn` _returnvalue_3) 0.0 "VTBlend_Linear" 0.0 false)
      (`/Game/Blueprints/GameplayActor/Second_Camera_Blueprint.The_Vision_Backwards` (`self.Camera`))
      (`KismetSystemLibrary.Delay` 3.0)
      (`Controller.SetIgnoreMoveInput` _returnvalue false)
      (`Controller.SetIgnoreLookInput` _returnvalue false)
      (bind _ashud_main_menu (cast `/Game/Menus/MainMenu/HUD_MainMenu` (`PlayerController.GetHUD` (`GameplayStatics.GetPlayerController` 0))))
      (`/Game/Menus/MainMenu/HUD_MainMenu.AddInterface` _ashud_main_menu))))

(fn `UserConstructionScript`)