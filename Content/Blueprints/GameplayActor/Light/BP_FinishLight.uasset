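; BP_FinishLight is a spotlight actor, presumably marking a finish point, that reacts to the player's distance.
; Every Tick it subtracts scaled distance to player 0 from base intensity and from the inner and outer cone angles, so the light dims and narrows as distance grows.
; An unconnected branch that would open every BP_LindasDoor once the player is close never runs.
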(event `self.ReceiveTick`
  (params (DeltaSeconds :type "Float (single-precision)"))
  (bind _returnvalue (`self.GetDistanceTo` (`GameplayStatics.GetPlayerCharacter` 0)))
  (bind _returnvalue_2 (/ _returnvalue (`self.DistanceConeDevider`)))
  (`|ExecutionSequence`
    (:`then_0`
      (`LightComponent.SetIntensity` (`self.SpotLightComponent`) (- (`self.Intensity`) (* _returnvalue (`self.DistanceMultieplier`)))))
    (:`then_1`
      (`SpotLightComponent.SetInnerConeAngle` (`self.SpotLightComponent`) (- (`self.InnerConeAngle`) _returnvalue_2)))
    (:`then_2`
      (`SpotLightComponent.SetOuterConeAngle` (`self.SpotLightComponent`) (- (`self.OuterConeAngle`) _returnvalue_2)))))

(fn `UserConstructionScript`)