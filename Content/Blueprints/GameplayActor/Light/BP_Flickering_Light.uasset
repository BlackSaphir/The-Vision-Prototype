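; Light actor that makes two spot lights and a point light flicker together once its Start_Flickering event is called.
; The event stores a random intensity multiplier and waits a short random delay, so timing and brightness can vary between triggers.
; It then plays the Flickering10s timeline, whose Flicker track, scaled by that multiplier, sets the intensity of all three lights on each update.
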(event `Start_Flickering`
  (set `self.Random ` (`KismetMathLibrary.RandomFloatInRange` 0.5 1.0))
  (`KismetSystemLibrary.Delay` (`KismetMathLibrary.RandomFloatInRange` 0.1 1.0))
  (bind (_direction _flicker) (`Timeline|Flickering 10s`)
    (:`Update`
      (`|ExecutionSequence`
        (:`then_0`
          (bind _returnvalue (* _flicker (`self.Random `)))
          (`LightComponent.SetIntensity` (`self.SpotLight`) _returnvalue))
        (:`then_1`
          (`LightComponent.SetIntensity` (`self.SpotLight1`) _returnvalue))
        (:`then_2`
          (`LightComponent.SetIntensity` (`self.PointLight`) _returnvalue))))))

(fn `UserConstructionScript`)