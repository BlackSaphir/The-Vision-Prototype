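; BP_LindasDoor is a three-panel door actor that toggles between open and closed each time BPEventActivate fires.
; A FlipFlop plays or reverses three timelines, which lerp the relative locations of the left, right and top panels between stored start and end vectors.
; The left panel uses the RightDoor vectors and vice versa.
; The door sound plays at world origin, once when opening and twice when closing.
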(event `ActivationInterface.BPEvent_Activate`
  (`/Engine/EditorBlueprintResources/StandardMacros.FlipFlop`
    (:`A`
      (`|ExecutionSequence`
        (:`then_0`
          (`GameplayStatics.PlaySoundAtLocation` "/Game/Audio/The_Vision_DoorOpenLong.The_Vision_DoorOpenLong")
          (bind (_direction _newtrack_1) (`Timeline|Timeline_0` :!label _label)
            (:`Update`
              (`SceneComponent.K2_SetRelativeLocation` (`self.DoorLeft`) (`KismetMathLibrary.VLerp` (`self.RightDoorStart`) (`self.RightDoorEnd`) _newtrack_1) false false))))
        (:`then_1`
          (bind (_direction_2 _newtrack_1_2) (`Timeline|Timeline_1` :!label _label_2)
            (:`Update`
              (`SceneComponent.K2_SetRelativeLocation` (`self.DoorRight`) (`KismetMathLibrary.VLerp` (`self.LeftDoorStart`) (`self.LeftDoorEnd`) _newtrack_1_2) false false))))
        (:`then_2`
          (bind (_direction_3 _newtrack_1_3) (`Timeline|Timeline_2` :!label _label_3)
            (:`Update`
              (`SceneComponent.K2_SetRelativeLocation` (`self.DoorTop`) (`KismetMathLibrary.VLerp` (`self.TopDoorStart`) (`self.TopDoorEnd`) _newtrack_1_3) false false))))))
    (:`B`
      (`|ExecutionSequence`
        (:`then_0`
          (goto _label :!via `Reverse`))
        (:`then_1`
          (`GameplayStatics.PlaySoundAtLocation` "/Game/Audio/The_Vision_DoorOpenLong.The_Vision_DoorOpenLong")
          (goto _label_2 :!via `Reverse`))
        (:`then_2`
          (`GameplayStatics.PlaySoundAtLocation` "/Game/Audio/The_Vision_DoorOpenLong.The_Vision_DoorOpenLong")
          (goto _label_3 :!via `Reverse`))))))

(fn `UserConstructionScript`)