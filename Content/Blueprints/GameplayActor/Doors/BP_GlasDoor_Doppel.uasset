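; BP_GlasDoor_Doppel is a double glass door with two leaves that swing open and closed when activated.
; BPEventActivate runs a FlipFlop that alternately plays and reverses two timelines, one per leaf.
; Each timeline lerps its leaf's relative rotation between start and end rotator variables.
; Separate OpenDoor and CloseDoor events snap both leaves to hardcoded rotations without animation, bypassing the FlipFlop and timelines.
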(event `ActivationInterface.BPEvent_Activate`
  (`/Engine/EditorBlueprintResources/StandardMacros.FlipFlop`
    (:`A`
      (`|ExecutionSequence`
        (:`then_0`
          (bind (_direction _newtrack_1) (`Timeline|Timeline_0` :!label _label)
            (:`Update`
              (`SceneComponent.K2_SetRelativeRotation` (`self.DoorLeft`) (`KismetMathLibrary.RLerp` (`self.LeftDoorStart`) (`self.LeftDoorEnd`) _newtrack_1) false false))))
        (:`then_1`
          (bind (_direction_2 _newtrack_1_2) (`Timeline|Timeline_1` :!label _label_2)
            (:`Update`
              (`SceneComponent.K2_SetRelativeRotation` (`self.DoorRight`) (`KismetMathLibrary.RLerp` (`self.RightDoorStart`) (`self.RightDoorEnd`) _newtrack_1_2) false false))))))
    (:`B`
      (`|ExecutionSequence`
        (:`then_0`
          (goto _label :!via `Reverse`))
        (:`then_1`
          (goto _label_2 :!via `Reverse`))))))

(event `self.Open_Door`
  (`|ExecutionSequence`
    (:`then_0`
      (`SceneComponent.K2_SetRelativeRotation` (`self.DoorLeft`) (struct :`Yaw` 90.0) false false))
    (:`then_1`
      (`SceneComponent.K2_SetRelativeRotation` (`self.DoorRight`) (struct :`Yaw` 90.0) false false))))

(event `self.Close_Door`
  (`|ExecutionSequence`
    (:`then_0`
      (`SceneComponent.K2_SetRelativeRotation` (`self.DoorLeft`) (struct) false false))
    (:`then_1`
      (`SceneComponent.K2_SetRelativeRotation` (`self.DoorRight`) (struct :`Yaw` 180.0) false false))))

(fn `UserConstructionScript`)