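; Two-panel sliding door actor that toggles between open and closed each time BPEventActivate or OpenDoor fires.
; A FlipFlop alternately plays and reverses two timelines, which lerp the panels' relative locations and play a door sound at world origin on each toggle.
; The variable names are crossed: LeftDoor moves between the RightDoor start/end vectors and RightDoor between the LeftDoor ones.
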(event `ActivationInterface.BPEvent_Activate`
  (`/Engine/EditorBlueprintResources/StandardMacros.FlipFlop` :!label _label
    (:`A`
      (`|ExecutionSequence`
        (:`then_0`
          (`GameplayStatics.PlaySoundAtLocation` "/Game/Audio/The_Vision_DoorOpenLong.The_Vision_DoorOpenLong")
          (bind (_direction _newtrack_1) (`Timeline|OpenSlideDoor` :!label _label_2)
            (:`Update`
              (`SceneComponent.K2_SetRelativeLocation` (`self.LeftDoor`) (`KismetMathLibrary.VLerp` (`self.RightDoorEnd`) (`self.RightDoorStart`) _newtrack_1) false false))))
        (:`then_1`
          (bind (_direction_2 _newtrack_1_2) (`Timeline|Timeline_0` :!label _label_3)
            (:`Update`
              (`SceneComponent.K2_SetRelativeLocation` (`self.RightDoor`) (`KismetMathLibrary.VLerp` (`self.LeftDoorEnd`) (`self.LeftDoorStart`) _newtrack_1_2) false false))))))
    (:`B`
      (`|ExecutionSequence`
        (:`then_0`
          (goto _label_2 :!via `Reverse`))
        (:`then_1`
          (`GameplayStatics.PlaySoundAtLocation` "/Game/Audio/The_Vision_DoorOpenLong.The_Vision_DoorOpenLong")
          (goto _label_3 :!via `Reverse`))))))

(event `OpenDoor`
  (goto _label))

(fn `UserConstructionScript`)