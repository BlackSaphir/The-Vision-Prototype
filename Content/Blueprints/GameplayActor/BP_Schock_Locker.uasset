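; BP_Schock_Locker is a locker actor whose door swings and slams once when the player comes near, apparently as a scare.
; Each Tick it checks the distance to the FirstPersonCharacter, and coming within range fires a DoOnce that plays a timeline.
; The timeline lerps the door's relative rotation between the Startrot and Endrot variables, then plays a loud, pitched-down slam sound at the locker when finished.
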(event `self.ReceiveTick`
  (params (DeltaSeconds :type "Float (single-precision)"))
  (bind _asfirst_person_character (cast `/Game/Blueprints/Character/FirstPersonCharacter` (`GameplayStatics.GetPlayerCharacter` 0)))
  (if (<= (`self.GetDistanceTo` _asfirst_person_character) 800.0)
    (`/Engine/EditorBlueprintResources/StandardMacros.DoOnce` false
      (:`Completed`
        (bind (_direction _newtrack_0) (`Timeline|Timeline_0`)
          (:`Update`
            (`SceneComponent.K2_SetRelativeRotation` (`self.Door`) (`KismetMathLibrary.RLerp` (`self.startrot`) (`self.endrot`) _newtrack_0) false false))
          (:`Finished`
            (`GameplayStatics.PlaySoundAtLocation` "/Game/Audio/118506__eddy15__locker-slam_CUT.118506__eddy15__locker-slam_CUT" (`SceneComponent.K2_GetComponentLocation` (`self.locker`)) (struct) 3.0 0.8)))))))

(fn `UserConstructionScript`)