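; BP_Sirene is a siren actor that shows a rotating spotlight and plays audio while IsActivated is true.
; Tick polls that flag, starting the audio once and spinning the SpotLight in yaw at a constant, frame-rate-independent speed.
; When the flag is false, a second DoOnce turns the light intensity to zero and stops the audio.
; Neither DoOnce is reset and the intensity is never restored, so each transition runs only once.
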(event `self.ReceiveTick`
  (params (DeltaSeconds :type "Float (single-precision)"))
  (if (`self.IsActivated`)
    (`|ExecutionSequence`
      (:`then_0`
        (`/Engine/EditorBlueprintResources/StandardMacros.DoOnce` false
          (:`Completed`
            (`AudioComponent.Play` (`self.Audio`) 0.0))))
      (:`then_1`
        (`SceneComponent.K2_AddLocalRotation` (`self.SpotLight`) (`KismetMathLibrary.MakeRotator` 0.0 0.0 (* DeltaSeconds 400.0)) false false)))
    (else
      (`/Engine/EditorBlueprintResources/StandardMacros.DoOnce` false
        (:`Completed`
          (`LightComponent.SetIntensity` (`self.SpotLight`) 0.0)
          (`AudioComponent.Stop` (`self.Audio`)))))))

(fn `UserConstructionScript`)