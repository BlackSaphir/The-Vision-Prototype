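; A trigger box that plays a one-shot timed camera cutaway when something overlaps it.
; On overlap it locks move and look input, clears all widgets, plays a view-change sound, starts the spotlights flickering and switches the view to a camera with its own ambience.
; After a fixed delay it plays the camera's exit sound, returns the view to the controlled pawn, unlocks input and restores the character's widgets.
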(event `self.CollisionComponent.OnComponentBeginOverlap`
  (params (OverlappedComponent :type "PrimitiveComponent Object Reference") (OtherActor :type "Actor Object Reference") (OtherComp :type "PrimitiveComponent Object Reference") (OtherBodyIndex :type Integer) (bFromSweep :type Boolean) (SweepResult :type "HitResult Structure (by ref)"))
  (bind _returnvalue (`GameplayStatics.GetPlayerController` 0))
  (bind _returnvalue_2 (`GameplayStatics.GetPlayerController` 0))
  (bind _returnvalue_3 (`GameplayStatics.GetPlayerController` 0))
  (`/Engine/EditorBlueprintResources/StandardMacros.DoOnce` false
    (:`Completed`
      (`Controller.SetIgnoreMoveInput` _returnvalue_2 true)
      (`Controller.SetIgnoreLookInput` _returnvalue_2 true)
      (`WidgetLayoutLibrary.RemoveAllWidgets`)
      (`GameplayStatics.PlaySoundAtLocation` "/Game/Audio/The_Vision_ViewChange.The_Vision_ViewChange" (`SceneComponent.RelativeLocation` (`self.CollisionComponent`)))
      (`/Game/Blueprints/GameplayActor/BP_Flickering_Light.Start_Flickering` (`self.Spot_Lights`))
      (`PlayerController.SetViewTargetWithBlend` (`GameplayStatics.GetPlayerController` 0) (`self.Camera`) 0.0 "VTBlend_Linear" 0.0 false)
      (`/Game/Blueprints/GameplayActor/Second_Camera_Blueprint.Play_Ambience_Camera_ViewChange` (`self.Camera`))
      (`KismetSystemLibrary.Delay` 10.0)
      (`/Game/Blueprints/GameplayActor/Second_Camera_Blueprint.Play_ChangeOut_Sound` (`self.Camera`))
      (`PlayerController.SetViewTargetWithBlend` _returnvalue_3 (`Controller.K2_GetPawn` _returnvalue_3) 0.0 "VTBlend_Linear" 0.0 false)
      (`Controller.SetIgnoreMoveInput` _returnvalue false)
      (`Controller.SetIgnoreLookInput` _returnvalue false)
      (`/Game/Blueprints/Character/FirstPersonCharacter.Add Widgets` (`self.Character`)))))

(fn `UserConstructionScript`)