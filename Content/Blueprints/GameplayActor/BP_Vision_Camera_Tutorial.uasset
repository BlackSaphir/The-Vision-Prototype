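; Camera actor for the tutorial's "Vision" effect, providing screen tint transitions and view-change sounds through events.
; Two timelines animate a uniform RGB scene color tint, one on a PostProcess component and one on the camera's own post-process settings.
; Each has a forward event and a reverse-from-end event.
; Separate events play the ambience and change-out sounds, positioned at the camera component's relative rather than world location.
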(event `Play_Ambience_Camera_ViewChange`
  (`GameplayStatics.PlaySoundAtLocation` "/Game/Audio/The_Vision_Ambience_Flackern_ViewChange.The_Vision_Ambience_Flackern_ViewChange" (`SceneComponent.RelativeLocation` (`self.CameraComponent`))))

(event `The_Vision`
  (bind (_direction _scene_color_tint) (`Timeline|Timeline_0` :`NewTime` 2.0 :!label _label)
    (:`Update`
      (set `PostProcessComponent.Settings` (make `PostProcessSettings` :`SceneColorTint` (make `LinearColor` _scene_color_tint _scene_color_tint _scene_color_tint 1.0)) (`self.PostProcess`)))))

(event `The_Vision_Backwards`
  (goto _label :!via `ReverseFromEnd`))

(event `inCamVision`
  (bind (_direction _scene_color_tint) (`Timeline|Timeline_1` :`NewTime` 2.0 :!via `PlayFromStart` :!label _label_2)
    (:`Update`
      (set `CameraComponent.PostProcessSettings` (make `PostProcessSettings` :`SceneColorTint` (make `LinearColor` _scene_color_tint _scene_color_tint _scene_color_tint 1.0)) (`self.CameraComponent`)))))

(event `Play_ChangeOut_Sound`
  (`GameplayStatics.PlaySoundAtLocation` "/Game/Audio/The_Vision_ViewChangeOut_2.The_Vision_ViewChangeOut_2" (`SceneComponent.RelativeLocation` (`self.CameraComponent`))))

(event `inCamBack`
  (goto _label_2 :!via `ReverseFromEnd`))

(fn `UserConstructionScript`)