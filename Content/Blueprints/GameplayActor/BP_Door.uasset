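; BP_Door is a sliding double door that opens and closes as actors pass through its Trigger component.
; Overlap begin toggles the DoorOpen flag at once, and overlap end runs the same toggle after a short delay, so the state flips rather than being set explicitly.
; The Animation timeline plays or reverses, lerping both leaves' relative locations between start and end positions.
; The Interaction event is an empty stub.
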(event `self.Trigger.OnComponentBeginOverlap`
  (params (OverlappedComponent :type "PrimitiveComponent Object Reference") (OtherActor :type "Actor Object Reference") (OtherComp :type "PrimitiveComponent Object Reference") (OtherBodyIndex :type Integer) (bFromSweep :type Boolean) (SweepResult :type "HitResult Structure (by ref)"))
  (if (`self.doorOpen`) :!label _label
    (set `self.doorOpen` false)
    (bind (_direction _animationtrack) (`Timeline|Animation` :!via `Reverse` :!label _label_2)
      (:`Update`
        (`|ExecutionSequence`
          (:`then_0`
            (`SceneComponent.K2_SetRelativeLocation` (`self.LeftDoor`) (`KismetMathLibrary.VLerp` (`self.StartPosLeftDoor`) (`self.EndPosLeftDoor`) _animationtrack) false false))
          (:`then_1`
            (`SceneComponent.K2_SetRelativeLocation` (`self.RightDoor`) (`KismetMathLibrary.VLerp` (`self.StartPosRightDoor`) (`self.EndPosRightDoor`) _animationtrack) false false)))))
    (else
      (set `self.doorOpen` true)
      (goto _label_2))))

(event `self.Trigger.OnComponentEndOverlap`
  (params (OverlappedComponent :type "PrimitiveComponent Object Reference") (OtherActor :type "Actor Object Reference") (OtherComp :type "PrimitiveComponent Object Reference") (OtherBodyIndex :type Integer))
  (`KismetSystemLibrary.Delay` 1.0)
  (goto _label))

(event `Interaction`)

(fn `UserConstructionScript`)