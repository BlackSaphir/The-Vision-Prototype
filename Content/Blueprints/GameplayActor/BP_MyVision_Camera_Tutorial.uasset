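; Tutorial variant of the MyVision camera actor, providing scene tint transitions and view-change sounds through custom events.
; Two timelines, each played forward or in reverse, drive a uniform RGB scene color tint: one on PostProcess settings, the other on the CameraComponent's own post-process settings.
; Separate events play flicker ambience and view-change-out sounds, using the camera component's relative location as the sound position.
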(event `CustomEvent_5`
  (`GameplayStatics.PlaySoundAtLocation` "/Game/Audio/The_Vision_Ambience_Flackern_ViewChange.The_Vision_Ambience_Flackern_ViewChange" (`SceneComponent.RelativeLocation` (`self.CameraComponent`))))

(event `CustomEvent`
  (bind (_direction _scene_color_tint) (`Timeline|Timeline_0` :`NewTime` 2.0 :!label _label)
    (:`Update`
      (set `PostProcessComponent.Settings` (make `PostProcessSettings` :`SceneColorTint` (make `LinearColor` _scene_color_tint _scene_color_tint _scene_color_tint 1.0)) (`self.PostProcess`)))))

(event `CustomEvent_1`
  (goto _label :!via `ReverseFromEnd`))

(event `CustomEvent_4`
  (`GameplayStatics.PlaySoundAtLocation` "/Game/Audio/The_Vision_ViewChangeOut_2.The_Vision_ViewChangeOut_2" (`SceneComponent.RelativeLocation` (`self.CameraComponent`))))

(event `CustomEvent_2`
  (bind (_direction _scene_color_tint) (`Timeline|Timeline_1` :`NewTime` 2.0 :!via `PlayFromStart` :!label _label_2)
    (:`Update`
      (set `CameraComponent.PostProcessSettings` (make `PostProcessSettings` :`SceneColorTint` (make `LinearColor` _scene_color_tint _scene_color_tint _scene_color_tint 1.0)) (`self.CameraComponent`)))))

(event `CustomEvent_3`
  (goto _label_2 :!via `ReverseFromEnd`))

(fn `UserConstructionScript`)