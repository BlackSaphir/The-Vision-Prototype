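; Camera actor for the "Vision" view, exposing events that fade scene color tint and play view-change sounds.
; TheVision and TheVisionBackwards run a timeline forward or in reverse to drive the PostProcess settings' tint.
; InCamVision and InCamBack do the same with a second timeline on the CameraComponent's own post-process settings.
; Separate events play ambience and change-out sounds, positioned using the camera component's relative location.
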(event `self.Play_Ambience_Camera_ViewChange`
  (`GameplayStatics.PlaySoundAtLocation` "/Game/Audio/Ambience/The_Vision_Ambience_Flackern_ViewChange.The_Vision_Ambience_Flackern_ViewChange" (`SceneComponent.RelativeLocation` (`self.CameraComponent`))))

(event `self.The_Vision`
  (bind (_direction _scene_color_tint) (`Timeline|Timeline_0` :`NewTime` 2.0 :!label _label)
    (:`Update`
      (set `PostProcessComponent.Settings` (make `PostProcessSettings` :`SceneColorTint` (make `LinearColor` _scene_color_tint _scene_color_tint _scene_color_tint 1.0)) (`self.PostProcess`)))))

(event `self.The_Vision_Backwards`
  (goto _label :!via `ReverseFromEnd`))

(event `self.InCamVision`
  (bind (_direction _scene_color_tint) (`Timeline|Timeline_1` :`NewTime` 2.0 :!via `PlayFromStart` :!label _label_2)
    (:`Update`
      (set `CameraComponent.PostProcessSettings` (make `PostProcessSettings` :`SceneColorTint` (make `LinearColor` _scene_color_tint _scene_color_tint _scene_color_tint 1.0)) (`self.CameraComponent`)))))

(event `self.Play_ChangeOut_Sound`
  (`GameplayStatics.PlaySoundAtLocation` "/Game/Audio/Effects/The_Vision_ViewChangeOut_2.The_Vision_ViewChangeOut_2" (`SceneComponent.RelativeLocation` (`self.CameraComponent`))))

(event `self.InCamBack`
  (goto _label_2 :!via `ReverseFromEnd`))

(fn `UserConstructionScript`)