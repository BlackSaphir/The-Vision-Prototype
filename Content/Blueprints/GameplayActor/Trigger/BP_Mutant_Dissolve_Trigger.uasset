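; BP_Mutant_Dissolve_Trigger is a one-shot overlap trigger that stages a scripted mutant scare.
; On first overlap it disables player input, resets the FirstPersonCharacter's inputs, starts tagged lights flickering and starts the tagged BP_Mutant_Dissolve dissolving.
; After a delay it briefly spawns a BP_Mutant_Enemy at a hardcoded transform with a scare sound, then destroys it and restores input.
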(event `self.Box.OnComponentBeginOverlap`
  (params (OverlappedComponent :type "PrimitiveComponent Object Reference") (OtherActor :type "Actor Object Reference") (OtherComp :type "PrimitiveComponent Object Reference") (OtherBodyIndex :type Integer) (bFromSweep :type Boolean) (SweepResult :type "HitResult Structure (by ref)"))
  (bind _returnvalue (`GameplayStatics.GetPlayerController` 0))
  (bind _returnvalue_2 (`GameplayStatics.GetPlayerController` 0))
  (bind _returnvalue_3 (`Controller.K2_GetPawn` _returnvalue_2))
  (`/Engine/EditorBlueprintResources/StandardMacros.DoOnce` false
    (:`Completed`
      (`self.DisableInput` _returnvalue_3 _returnvalue_2)
      (bind _asfirst_person_character (cast `/Game/Blueprints/Character/FirstPersonCharacter` _returnvalue_3))
      (`The_VisionCharacter.ResetInputs` _asfirst_person_character)
      (bind _outactors (`GameplayStatics.GetAllActorsWithTag` "Flickering_Light_Mutant"))
      (for _array_element _outactors
        (bind _output_get (set `self.Flickering_Light` (`|MakeArray` (cast `/Game/Blueprints/GameplayActor/Light/BP_Flickering_Light` _array_element :!pure true))))
        (`/Game/Blueprints/GameplayActor/Light/BP_Flickering_Light.Start_Flickering` _output_get))
      (bind _outactors_2 (`GameplayStatics.GetAllActorsWithTag` "Mutant_Dissolve"))
      (bind _output_get_2 (set `self.Mutant` (cast `/Game/Blueprints/AI/BP_Mutant_Dissolve` (`|GetArrayItem` _outactors_2) :!pure true)))
      (`/Game/Blueprints/AI/BP_Mutant_Dissolve.Start_Dissolve` _output_get_2)
      (`KismetSystemLibrary.Delay` 5.2)
      (bind _returnvalue_4 (`|SpawnActorFromClass` "/Game/Blueprints/AI/BP_Mutant_Enemy.BP_Mutant_Enemy_C" (`KismetMathLibrary.MakeTransform` (6568.0 -1885.0 254.000107) (struct :`Yaw` -90.0)) "Undefined" "OverrideRootScale" null null))
      (`GameplayStatics.PlaySoundAtLocation` "/Game/Audio/Effects/The_Vision_ScarySound.The_Vision_ScarySound" (`self.K2_GetActorLocation` (`GameplayStatics.GetPlayerController` 0)) (struct) 1.5)
      (`KismetSystemLibrary.Delay` 1.0)
      (`self.K2_DestroyActor` _returnvalue_4)
      (`self.EnableInput` (`Controller.K2_GetPawn` _returnvalue) _returnvalue))))

(fn `UserConstructionScript`)