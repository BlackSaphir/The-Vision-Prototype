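; One-shot overlap trigger that plays the Vision tutorial sequence, temporarily moving the player's view to a tagged tutorial camera.
; It disables input, clears widgets, plays blur emitters and sounds, flags tutorial AI spawn points, then blends to the camera.
; During the vision, enemies get custom-depth stencil highlighting and "Hide" actors disappear.
; Timed delays then restore the view, visibility, input and HUD, and destroy the tagged tutorial sphere.
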(event `self.CollisionComponent.OnComponentBeginOverlap`
  (params (OverlappedComponent :type "PrimitiveComponent Object Reference") (OtherActor :type "Actor Object Reference") (OtherComp :type "PrimitiveComponent Object Reference") (OtherBodyIndex :type Integer) (bFromSweep :type Boolean) (SweepResult :type "HitResult Structure (by ref)"))
  (bind _returnvalue (`GameplayStatics.GetPlayerController` 0))
  (bind _returnvalue_2 (`GameplayStatics.GetPlayerController` 0))
  (bind _returnvalue_3 (`GameplayStatics.GetPlayerController` 0))
  (bind _camera (`self.Camera`))
  (bind _camera_2 (`self.Camera`))
  (`/Engine/EditorBlueprintResources/StandardMacros.DoOnce` false
    (:`Completed`
      (bind _outactors (`GameplayStatics.GetAllActorsWithTag` "Vision_Trigger_Tutorial"))
      (set `self.Camera` (cast `/Game/Blueprints/GameplayActor/BP_Vision_Camera_Tutorial` (`|GetArrayItem` _outactors) :!pure true))
      (`self.DisableInput` (`Controller.K2_GetPawn` _returnvalue_2) _returnvalue_2)
      (bind _asfirst_person_character (cast `/Game/Blueprints/Character/FirstPersonCharacter` (`GameplayStatics.GetPlayerCharacter` 0)))
      (`The_VisionCharacter.ResetInputs` _asfirst_person_character)
      (`WidgetLayoutLibrary.RemoveAllWidgets`)
      (`GameplayStatics.PlaySoundAtLocation` "/Game/Audio/The_Vision_ViewChange.The_Vision_ViewChange" (`SceneComponent.RelativeLocation` (`self.CollisionComponent`)))
      (`|ExecutionSequence`
        (:`then_0`
          (`KismetSystemLibrary.Delay` 1.5)
          (`/Game/Blueprints/GameplayActor/BP_Vision_Camera_Tutorial.The_Vision` (`self.Camera`))
          (bind _outactors_2 (`GameplayStatics.GetAllActorsOfClass` "/Game/Blueprints/AI/AI_SpawnPoint_Tutorial.AI_SpawnPoint_Tutorial_C"))
          (`KismetSystemLibrary.Delay` 1.0)
          (`/Game/Blueprints/AI/AI_SpawnPoint_Tutorial.SetSpawnBoolTrue_Tutorial` _outactors_2)
          (`PlayerController.SetViewTargetWithBlend` (`GameplayStatics.GetPlayerController` 0) (`self.Camera`) 0.0 "VTBlend_Linear" 0.0 false)
          (`KismetSystemLibrary.Delay` 0.0)
          (`/Game/Blueprints/GameplayActor/BP_Vision_Camera_Tutorial.inCamVision` _camera_2)
          (`/Game/Blueprints/GameplayActor/BP_Vision_Camera_Tutorial.Play_Ambience_Camera_ViewChange` _camera_2)
          (`|ExecutionSequence`
            (:`then_0`
              (`KismetSystemLibrary.Delay` 10.0)
              (`/Game/Blueprints/GameplayActor/BP_Vision_Camera_Tutorial.Play_ChangeOut_Sound` _camera)
              (`/Game/Blueprints/GameplayActor/BP_Vision_Camera_Tutorial.inCamBack` _camera)
              (`KismetSystemLibrary.Delay` 2.0)
              (`PlayerController.SetViewTargetWithBlend` _returnvalue_3 (`Controller.K2_GetPawn` _returnvalue_3) 0.0 "VTBlend_Linear" 0.0 false)
              (`KismetSystemLibrary.Delay` 0.0)
              (`/Game/Blueprints/GameplayActor/BP_Vision_Camera_Tutorial.The_Vision_Backwards` (`self.Camera`))
              (`|ExecutionSequence`
                (:`then_0`
                  (`KismetSystemLibrary.Delay` 4.0)
                  (`self.EnableInput` (`Controller.K2_GetPawn` _returnvalue) _returnvalue)
                  (bind _ashud_main_menu (cast `/Game/Menus/MainMenu/HUD_MainMenu` (`PlayerController.GetHUD` (`GameplayStatics.GetPlayerController` 0))))
                  (`/Game/Menus/MainMenu/HUD_MainMenu.AddInterface` _ashud_main_menu)
                  (bind _outactors_3 (`GameplayStatics.GetAllActorsWithTag` "The_Vision_Tutorial_Sphere"))
                  (`self.K2_DestroyActor` _outactors_3))
                (:`then_1`
                  (bind _asthe_vision_character (cast `The_VisionCharacter` (`Controller.K2_GetPawn` (`GameplayStatics.GetPlayerController` 0))))
                  (bind _returnvalue_4 (`GameplayStatics.SpawnEmitterAttached` "/Game/Objects/Level_Objects/Materials/Camera/P_Vision_Blur_back.P_Vision_Blur_back" (`The_VisionCharacter.FirstPersonCamera` _asthe_vision_character) "None" (0.0 0.0 0.0) (struct) "SnapToTarget"))
                  (`KismetSystemLibrary.Delay` 4.0)
                  (`ActorComponent.K2_DestroyComponent` _returnvalue_4))
                (:`then_2`
                  (bind _outactors_4 (`GameplayStatics.GetAllActorsOfClass` "/Game/Blueprints/AI/Enemy_Character_BP.Enemy_Character_BP_C"))
                  (for _array_element _outactors_4
                    (`PrimitiveComponent.SetRenderCustomDepth` (`Character.Mesh` _array_element) false)))
                (:`then_3`
                  (bind _outactors_5 (`GameplayStatics.GetAllActorsWithTag` "Hide"))
                  (for _array_element_2 _outactors_5
                    (`self.SetActorHiddenInGame` _array_element_2 false)))))
            (:`then_1`
              (bind _outactors_6 (`GameplayStatics.GetAllActorsOfClass` "/Game/Blueprints/AI/Enemy_Character_BP.Enemy_Character_BP_C"))
              (for _array_element_3 _outactors_6
                (bind _mesh (`Character.Mesh` _array_element_3))
                (`PrimitiveComponent.SetRenderCustomDepth` _mesh true)
                (`PrimitiveComponent.SetCustomDepthStencilValue` _mesh 254)))
            (:`then_2`
              (bind _outactors_7 (`GameplayStatics.GetAllActorsWithTag` "Hide"))
              (for _array_element_4 _outactors_7
                (`self.SetActorHiddenInGame` _array_element_4 true)))))
        (:`then_1`
          (bind _asthe_vision_character_2 (cast `The_VisionCharacter` (`Controller.K2_GetPawn` (`GameplayStatics.GetPlayerController` 0))))
          (bind _returnvalue_5 (`GameplayStatics.SpawnEmitterAttached` "/Game/Objects/Level_Objects/Materials/Camera/P_Vision_Blur.P_Vision_Blur" (`The_VisionCharacter.FirstPersonCamera` _asthe_vision_character_2) "None" (0.0 0.0 0.0) (struct) "SnapToTarget"))
          (`KismetSystemLibrary.Delay` 2.0)
          (`ActorComponent.K2_DestroyComponent` _returnvalue_5))))))

(fn `UserConstructionScript`)