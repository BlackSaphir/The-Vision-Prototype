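; One-shot trigger volume that sends the player into the nightmare through a blurred vision transition.
; On first overlap it disables and resets input, removes all widgets, plays the view-change sound and attaches a blur particle to the Vision character's camera.
; After a short delay it teleports the player to a hardcoded position and rotation, removes the blur, re-enables input and restores the HUD interface.
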(event `self.CollisionComponent.OnComponentBeginOverlap`
  (params (OverlappedComponent :type "PrimitiveComponent Object Reference") (OtherActor :type "Actor Object Reference") (OtherComp :type "PrimitiveComponent Object Reference") (OtherBodyIndex :type Integer) (bFromSweep :type Boolean) (SweepResult :type "HitResult Structure (by ref)"))
  (bind _returnvalue (`GameplayStatics.GetPlayerController` 0))
  (bind _returnvalue_2 (`GameplayStatics.GetPlayerController` 0))
  (`/Engine/EditorBlueprintResources/StandardMacros.DoOnce` false
    (:`Completed`
      (`self.DisableInput` (`Controller.K2_GetPawn` _returnvalue_2) _returnvalue_2)
      (bind _asfirst_person_character (cast `/Game/Blueprints/Character/FirstPersonCharacter` (`GameplayStatics.GetPlayerCharacter` 0)))
      (`The_VisionCharacter.ResetInputs` _asfirst_person_character)
      (`WidgetLayoutLibrary.RemoveAllWidgets`)
      (`GameplayStatics.PlaySoundAtLocation` "/Game/Audio/The_Vision_ViewChange.The_Vision_ViewChange" (`SceneComponent.RelativeLocation` (`self.CollisionComponent`)))
      (bind _asthe_vision_character (cast `The_VisionCharacter` (`Controller.K2_GetPawn` (`GameplayStatics.GetPlayerController` 0))))
      (bind _returnvalue_3 (`GameplayStatics.SpawnEmitterAttached` "/Game/Objects/Level_Objects/Materials/Camera/P_Vision_Blur.P_Vision_Blur" (`The_VisionCharacter.FirstPersonCamera` _asthe_vision_character) "None" (0.0 0.0 0.0) (struct) "SnapToTarget"))
      (`KismetSystemLibrary.Delay` 4.0)
      (bind _asfirst_person_character_2 (cast `/Game/Blueprints/Character/FirstPersonCharacter` (`GameplayStatics.GetPlayerCharacter` 0)))
      (`self.K2_SetActorLocationAndRotation` _asfirst_person_character_2 (8222.000977 -1627.000732 198.0) (struct :`Yaw` 90.0) false false)
      (`ActorComponent.K2_DestroyComponent` _returnvalue_3)
      (`self.EnableInput` (`Controller.K2_GetPawn` _returnvalue) _returnvalue)
      (bind _ashud_main_menu (cast `/Game/Menus/MainMenu/HUD_MainMenu` (`PlayerController.GetHUD` (`GameplayStatics.GetPlayerController` 0))))
      (`/Game/Menus/MainMenu/HUD_MainMenu.AddInterface` _ashud_main_menu))))

(fn `UserConstructionScript`)