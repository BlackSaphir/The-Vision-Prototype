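; BP_Interact_Trigger is a box trigger that flags the first-person player as being inside an interaction zone.
; Begin overlap casts player 0's controlled pawn, without checking the overlapping actor, caches it and sets its InTrigger flag.
; End overlap clears the flag on that cached character, likewise for any actor leaving the box.
; BeginPlay creates and stores a Bp_Interact widget, which this graph never displays.
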(event `self.ReceiveBeginPlay`
  (bind _returnvalue (`|CreateWidget` "/Game/Blueprints/Widgets/Bp_Interact.Bp_Interact_C"))
  (set `self.InteractWidget` _returnvalue))

(event `self.Box.OnComponentBeginOverlap`
  (params (OverlappedComponent :type "PrimitiveComponent Object Reference") (OtherActor :type "Actor Object Reference") (OtherComp :type "PrimitiveComponent Object Reference") (OtherBodyIndex :type Integer) (bFromSweep :type Boolean) (SweepResult :type "HitResult Structure (by ref)"))
  (bind _asfirst_person_character (cast `/Game/Blueprints/Character/FirstPersonCharacter` (`Controller.K2_GetPawn` (`GameplayStatics.GetPlayerController` 0))))
  (set `self.FPSRef` _asfirst_person_character)
  (set `/Game/Blueprints/Character/FirstPersonCharacter.bInTrigger` true (`self.FPSRef`)))

(event `self.Box.OnComponentEndOverlap`
  (params (OverlappedComponent :type "PrimitiveComponent Object Reference") (OtherActor :type "Actor Object Reference") (OtherComp :type "PrimitiveComponent Object Reference") (OtherBodyIndex :type Integer))
  (`/Engine/EditorBlueprintResources/StandardMacros.IsValid` (`self.FPSRef`)
    (:`Is Valid`
      (set `/Game/Blueprints/Character/FirstPersonCharacter.bInTrigger` false (`self.FPSRef`)))))

(fn `UserConstructionScript`)