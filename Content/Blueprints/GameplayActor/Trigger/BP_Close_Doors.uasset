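; Trigger actor that runs a one-time, timed sequence on two tutorial slide doors when its box is first overlapped.
; It finds the first actor under each of two tags and casts it to BP_SlideDoorNicoOpen.
; A chain of delays staggers repeated OpenDoor calls on both doors, with no separate close call despite the asset's name.
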(event `self.Box.OnComponentBeginOverlap`
  (params (OverlappedComponent :type "PrimitiveComponent Object Reference") (OtherActor :type "Actor Object Reference") (OtherComp :type "PrimitiveComponent Object Reference") (OtherBodyIndex :type Integer) (bFromSweep :type Boolean) (SweepResult :type "HitResult Structure (by ref)"))
  (`/Engine/EditorBlueprintResources/StandardMacros.DoOnce` false
    (:`Completed`
      (bind _outactors (`GameplayStatics.GetAllActorsWithTag` "Slide_Door_Tutorial"))
      (bind _asbp_slide_door_nico_open (cast `/Game/Blueprints/GameplayActor/Doors/BP_SlideDoorNicoOpen` (`|GetArrayItem` _outactors) :!pure true))
      (set `self.Slide_Door_Tutorial_1` _asbp_slide_door_nico_open)
      (`/Game/Blueprints/GameplayActor/Doors/BP_SlideDoorNicoOpen.OpenDoor` _asbp_slide_door_nico_open)
      (`KismetSystemLibrary.Delay` 2.0)
      (bind _outactors_2 (`GameplayStatics.GetAllActorsWithTag` "Slide_Door_Tutorial_2"))
      (bind _output_get (set `self.Slide_Door_Tutorial_2` (cast `/Game/Blueprints/GameplayActor/Doors/BP_SlideDoorNicoOpen` (`|GetArrayItem` _outactors_2) :!pure true)))
      (`/Game/Blueprints/GameplayActor/Doors/BP_SlideDoorNicoOpen.OpenDoor` _output_get)
      (`KismetSystemLibrary.Delay` 6.5)
      (`/Game/Blueprints/GameplayActor/Doors/BP_SlideDoorNicoOpen.OpenDoor` (`self.Slide_Door_Tutorial_1`))
      (`/Game/Blueprints/GameplayActor/Doors/BP_SlideDoorNicoOpen.OpenDoor` (`self.Slide_Door_Tutorial_2`))
      (`KismetSystemLibrary.Delay` 4.5)
      (`/Game/Blueprints/GameplayActor/Doors/BP_SlideDoorNicoOpen.OpenDoor` (`self.Slide_Door_Tutorial_1`))
      (`KismetSystemLibrary.Delay` 1.5)
      (`/Game/Blueprints/GameplayActor/Doors/BP_SlideDoorNicoOpen.OpenDoor` (`self.Slide_Door_Tutorial_2`)))))

(fn `UserConstructionScript`)