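; A level streaming trigger volume for Laboratory 1 that swaps sublevels as the player moves through it.
; When the player character enters the Box, it loads the lab level, visible on load and blocking until finished.
; When the player leaves, it unloads the EDV and pause room levels, with all level names taken from variables.
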(event `self.Box.OnComponentBeginOverlap`
  (params (OverlappedComponent :type "PrimitiveComponent Object Reference") (OtherActor :type "Actor Object Reference") (OtherComp :type "PrimitiveComponent Object Reference") (OtherBodyIndex :type Integer) (bFromSweep :type Boolean) (SweepResult :type "HitResult Structure (by ref)"))
  (if (== OtherActor (`GameplayStatics.GetPlayerCharacter` 0))
    (`GameplayStatics.LoadStreamLevel` (`self.Level_to_Stream_Lab`) true true)))

(event `self.Box.OnComponentEndOverlap`
  (params (OverlappedComponent :type "PrimitiveComponent Object Reference") (OtherActor :type "Actor Object Reference") (OtherComp :type "PrimitiveComponent Object Reference") (OtherBodyIndex :type Integer))
  (if (== OtherActor (`GameplayStatics.GetPlayerCharacter` 0))
    (`GameplayStatics.UnloadStreamLevel` (`self.Level_to_Unload_EDV`))
    (`GameplayStatics.UnloadStreamLevel` (`self.Level_to_Unload_PauseRoom`))))

(fn `UserConstructionScript`)