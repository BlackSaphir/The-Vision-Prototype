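; BP_AlarmButton is an alarm button actor that switches off every BP_Sirene in the level when activated.
; Tick checks the distance to the FirstPersonCharacter, highlighting the unpressed button through custom depth stencil when near and clearing it when far.
; BPEventActivate clears IsActivated on each siren found, marks the button pressed and removes the highlight, all inside the loop, so only if a siren exists.
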(event `self.ReceiveTick`
  (params (DeltaSeconds :type "Float (single-precision)"))
  (bind _asfirst_person_character (cast `/Game/Blueprints/Character/FirstPersonCharacter` (`GameplayStatics.GetPlayerCharacter` 0)))
  (`/Engine/EditorBlueprintResources/StandardMacros.IsValid` _asfirst_person_character
    (:`Is Valid`
      (`/Engine/EditorBlueprintResources/StandardMacros.CompareFloat` (`self.GetDistanceTo` _asfirst_person_character) 500.0
        (:`>`
          (`PrimitiveComponent.SetRenderCustomDepth` (`self.Button`) false))
        (:`<`
          (if (not (`self.ButtonPressed`))
            (`PrimitiveComponent.SetCustomDepthStencilValue` (`self.Button`) 252)
            (`PrimitiveComponent.SetRenderCustomDepth` (`self.Button`) true)))))))

(event `self.ReceiveBeginPlay`
  (`PrimitiveComponent.SetRenderCustomDepth` (`self.Button`) false))

(event `ActivationInterface.BPEvent_Activate`
  (bind _outactors (`GameplayStatics.GetAllActorsOfClass` "/Game/Blueprints/GameplayActor/BP_Sirene.BP_Sirene_C"))
  (for _array_element _outactors
    (set `/Game/Blueprints/GameplayActor/BP_Sirene.IsActivated` false _array_element)
    (set `self.ButtonPressed` true)
    (`PrimitiveComponent.SetRenderCustomDepth` (`self.Button`) false)))

(fn `UserConstructionScript`)